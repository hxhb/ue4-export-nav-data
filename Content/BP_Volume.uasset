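; Box volume tool for exporting navmesh data and debug-testing pathfinding between BeginActor and EndActor.
; Construction script sizes the box and offsets Min/Max markers, whose bounds ExportNav writes to a file.
; FindPath events query engine navigation or load saved files through DtNavMeshWrapper for Detour queries, printing and drawing results.
; The engine test branches on an unexecuted Detour call's result; GenerateAStartTiles is an unfinished floor-trace stub.
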(event Custom|ExportNav
  (bind (_min _max) (CallFunction|GetPoints))
  (bind _savepath (Variables|Export|GetSavePath))
  (bind _name (Variables|Export|GetName))
  (bind _path (Utilities|Struct|BreakDirectoryPath _savepath))
  (bind _array (Utilities|Array|MakeArray _path _name))
  (bind _returnvalue (Class|BlueprintPathsLibrary|Combine _array))
  (Class|FlibExportNevChunk|ExportNavAreabyRef 0 (Math|Box|MakeBox _min _max) _returnvalue)
  (Development|PrintString _returnvalue))

(event Custom|FindPath%28RecastNav%29
  (bind _beginactor (Variables|Nav|GetBeginActor))
  (bind _endactor (Variables|Nav|GetEndActor))
  (bind _returnvalue (Transformation|GetActorLocation _endactor))
  (bind _returnvalue_2 (Transformation|GetActorLocation _beginactor))
  (Utilities|IsValid _beginactor
    (:Is%20Valid
      (Utilities|IsValid _endactor
        (:Is%20Valid
          (Utilities|FlowControl|Sequence
            (:then_0
              (Development|PrintString "FindPath(RecastNav)" true true "(R=1.000000,G=0.000000,B=0.000000,A=1.000000)" 5.0))
            (:then_1
              (Development|PrintString (Utilities|String|Append "Satrt:" (Utilities|String|ToString(Vector) _returnvalue_2)) true true "(R=0.000000,G=0.660000,B=1.000000,A=1.000000)" 5.0)
              (Development|PrintString (Utilities|String|Append "End:" (Utilities|String|ToString(Vector) _returnvalue)) true true "(R=0.000000,G=0.660000,B=1.000000,A=1.000000)" 5.0))
            (:then_2
              (bind _returnvalue_3 (Game|ConstructObjectfromClass "/Script/ExportNavRuntime.dtNavMeshWrapper" self))
              (bind _output_get (Variables|Default|SetNavMeshWrapper _returnvalue_3))
              (Utilities|FlowControl|Sequence
                (:then_0
                  (Utilities|Array|Clear (Variables|Default|GetNavMeshPaths))
                  (for _array_element (Variables|Nav|GetNavMeshFile)
                    (Utilities|Array|AddUnique (Variables|Default|GetNavMeshPaths) (Utilities|Struct|BreakFilePath _array_element))
                    (Development|PrintString (Utilities|Struct|BreakFilePath _array_element) true true "(R=0.000000,G=0.660000,B=1.000000,A=1.000000)" 5.0)))
                (:then_1
                  (bind _returnvalue_4 (Class|DtNavMeshWrapper|LoadNavData _output_get (Variables|Default|GetNavMeshPaths)))
                  (Utilities|FlowControl|Sequence
                    (:then_0
                      (bind (_outpaths _returnvalue_5) (Class|FlibExportNavData|FindDetourPathfromGameAxisbyNavObject _returnvalue_4 _returnvalue_2 _returnvalue (Variables|Nav|GetExtern)))
                      (if _returnvalue_5
                        (for _array_element_2 _outpaths
                          (Development|PrintString (Utilities|String|ToString(Vector) _array_element_2) true true "(R=0.000000,G=0.660000,B=1.000000,A=1.000000)" 5.0)
                          (Rendering|Debug|DrawDebugSphere _array_element_2 1e+02 12 "(R=1.000000,G=0.000000,B=0.000000,A=1.000000)" 5.0))
                        (else
                          (Development|PrintString "FindPaht Faild!" true true "(R=0.000000,G=0.660000,B=1.000000,A=1.000000)" 5.0))))))))))))))

(event Custom|FindPath%28EngineNav%29
  (bind _beginactor (Variables|Nav|GetBeginActor))
  (bind _endactor (Variables|Nav|GetEndActor))
  (bind _returnvalue (Transformation|GetActorLocation _beginactor))
  (bind _returnvalue_2 (Transformation|GetActorLocation _endactor))
  (Utilities|IsValid _beginactor
    (:Is%20Valid
      (Utilities|IsValid _endactor
        (:Is%20Valid
          (Utilities|FlowControl|Sequence
            (:then_0
              (Development|PrintString "FindPath(EngineNav)" true true "(R=1.000000,G=0.000000,B=0.000000,A=1.000000)" 5.0))
            (:then_1
              (Development|PrintString (Utilities|String|Append "Satrt:" (Utilities|String|ToString(Vector) _returnvalue)) true true "(R=0.000000,G=0.660000,B=1.000000,A=1.000000)" 5.0)
              (Development|PrintString (Utilities|String|Append "End:" (Utilities|String|ToString(Vector) _returnvalue_2)) true true "(R=0.000000,G=0.660000,B=1.000000,A=1.000000)" 5.0))
            (:then_2
              (bind _returnvalue_3 (Class|NavigationSystemV1|FindPathtoLocationSynchronously _returnvalue _returnvalue_2 0 0))
              (if (stale _returnvalue)
                (for _array_element (Variables|/Script/NavigationSystem.NavigationPath|GetPathPoints _returnvalue_3)
                  (Development|PrintString (Utilities|String|ToString(Vector) _array_element) true true "(R=0.000000,G=0.660000,B=1.000000,A=1.000000)" 5.0)
                  (Rendering|Debug|DrawDebugSphere _array_element 1e+02 12 "(R=1.000000,G=0.000000,B=0.840064,A=1.000000)" 5.0))
                (else
                  (Development|PrintString "FindPaht Faild!" true true "(R=0.000000,G=0.660000,B=1.000000,A=1.000000)" 5.0))))))))))

(event Custom|GenerateAStartTiles
  (bind _max (Variables|Default|GetMax))
  (bind _max_2 (Variables|Default|GetMax))
  (bind _returnvalue (Transformation|GetWorldLocation _max))
  (bind _returnvalue_2 (Transformation|GetWorldLocation _max_2))
  (bind (_x _y _z) (Math|Vector|BreakVector _returnvalue))
  (bind (_x_2 _y_2 _z_2) (Math|Vector|BreakVector _returnvalue_2))
  (bind (_outhit _returnvalue_3) (Collision|LineTraceByChannel (Math|Vector|MakeVector _x_2 _y_2 (+ _z_2 5e+03)) (Math|Vector|MakeVector _x _y (- _z 1e+04)) "TraceTypeQuery1" false 0 "ForOneFrame"))
  (if _returnvalue_3
    (if (Actor|ActorHasTag (.HitActor (Collision|BreakHitResult _outhit)) "floor")
      _)))

(event EventBeginPlay)

(event Collision|EventActorBeginOverlap
  (params (OtherActor :type Actor%20Object%20Reference)))

(event EventTick
  (params (DeltaSeconds :type Float%20%28single-precision%29)))

(fn ConstructionScript
  (bind _box (Variables|Default|GetBox))
  (bind _returnvalue (Components|Box|GetScaledBoxExtent _box))
  (bind (_x _y _z) (Math|Vector|BreakVector _returnvalue))
  (bind (_x_2 _y_2 _z_2) (Math|Vector|BreakVector _returnvalue))
  (Components|Box|SetBoxExtent (Variables|Default|GetBox) (Variables|Export|GetBoxExtern) true)
  (Transformation|AddRelativeLocation (Variables|Default|GetMax) (Math|Vector|MakeVector _x _y _z) false false)
  (Transformation|AddRelativeLocation (Variables|Default|GetMin) (Math|Vector|MakeVector (- 0.0 _x_2) (- 0.0 _y_2) (- 0.0 _z_2)) false false))

(fn GetPoints
  (return (Transformation|GetWorldLocation (Variables|Default|GetMin)) (Transformation|GetWorldLocation (Variables|Default|GetMax))))